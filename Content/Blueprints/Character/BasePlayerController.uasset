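; Base player controller Blueprint that receives player input and relays it to the controlled pawn.
; It caches the pawn once on BeginPlay, then forwards each action and axis as a message call, leaving the gameplay logic to the pawn.
; Held actions send true on press and false on release, axes pass their values, weapon keys send a slot index, and Interact sends only on press.
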(event EventBeginPlay
  (Variables|Default|SetPlayerPawn (Pawn|GetControlledPawn)))

(event EventTick
  (params (DeltaSeconds :type Float%20%28single-precision%29)))

(event Input|ActionEvents|InputActionFire
  (params (Key :type Key%20Structure :default "None"))
  (bind _playerpawn (Variables|Default|GetPlayerPawn))
  ;[1 1 1] Inputs
  (:Pressed
    (Class|InputInterface|Shoot(Message) _playerpawn true))
  (:Released
    (Class|InputInterface|Shoot(Message) _playerpawn false)))

(event Input|ActionEvents|InputActionJump
  (params (Key :type Key%20Structure :default "None"))
  (bind _playerpawn (Variables|Default|GetPlayerPawn))
  ;[1 1 1] Inputs
  (:Pressed
    (Class|InputInterface|Leap(Message) _playerpawn true))
  (:Released
    (Class|InputInterface|Leap(Message) _playerpawn false)))

(event Input|ActionEvents|InputActionReload
  (params (Key :type Key%20Structure :default "None"))
  (bind _playerpawn (Variables|Default|GetPlayerPawn))
  ;[1 1 1] Inputs
  (:Pressed
    (Class|InputInterface|Reload(Message) _playerpawn true))
  (:Released
    (Class|InputInterface|Reload(Message) _playerpawn false)))

(event Input|ActionEvents|InputActionPunch
  (params (Key :type Key%20Structure :default "None"))
  (bind _playerpawn (Variables|Default|GetPlayerPawn))
  ;[1 1 1] Inputs
  (:Pressed
    (Class|InputInterface|Melee(Message) _playerpawn true))
  (:Released
    (Class|InputInterface|Melee(Message) _playerpawn false)))

(event Input|ActionEvents|InputActionCrouch
  (params (Key :type Key%20Structure :default "None"))
  (bind _playerpawn (Variables|Default|GetPlayerPawn))
  ;[1 1 1] Inputs
  (:Pressed
    (Class|InputInterface|Duck(Message) _playerpawn true))
  (:Released
    (Class|InputInterface|Duck(Message) _playerpawn false)))

(event Input|ActionEvents|InputActionPrimary
  (params (Key :type Key%20Structure :default "None"))
  ;[1 1 1] Inputs
  (:Pressed
    (Class|InputInterface|ChangeWeapon(Message) (Variables|Default|GetPlayerPawn))))

(event Input|ActionEvents|InputActionSecondary
  (params (Key :type Key%20Structure :default "None"))
  ;[1 1 1] Inputs
  (:Pressed
    (Class|InputInterface|ChangeWeapon(Message) (Variables|Default|GetPlayerPawn) 1)))

(event Input|ActionEvents|InputActionInteract
  (params (Key :type Key%20Structure :default "None"))
  ;[1 1 1] Inputs
  (:Pressed
    (Class|InputInterface|Interact(Message) (Variables|Default|GetPlayerPawn) true)))

(event Input|AxisEvents|InputAxisMoveForward
  (params (AxisValue :type Float%20%28single-precision%29))
  ;[1 1 1] Inputs
  (Class|InputInterface|ForwardInput(Message) (Variables|Default|GetPlayerPawn) AxisValue))

(event Input|AxisEvents|InputAxisMoveRight
  (params (AxisValue :type Float%20%28single-precision%29))
  ;[1 1 1] Inputs
  (Class|InputInterface|RightInput(Message) (Variables|Default|GetPlayerPawn) AxisValue))

(event Input|AxisEvents|InputAxisLookUp
  (params (AxisValue :type Float%20%28single-precision%29))
  ;[1 1 1] Inputs
  (Class|InputInterface|LookUp(Message) (Variables|Default|GetPlayerPawn) AxisValue))

(event Input|AxisEvents|InputAxisLookRight
  (params (AxisValue :type Float%20%28single-precision%29))
  ;[1 1 1] Inputs
  (Class|InputInterface|LookRight(Message) (Variables|Default|GetPlayerPawn) AxisValue))

(fn ConstructionScript)