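; Loot table component that spawns a pickup at its owning actor's location when SpawnLoot is called.
; SpawnLoot takes its class from ChooseLoot, which holds a random Select across armour, health, weapon and ammo categories.
; Nested weighted rolls favour smaller or more basic pickups within each category.
; The Select has no visible connection to an output, so the class ChooseLoot actually returns is unclear.
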(event EventBeginPlay)

(event EventTick
  (params (DeltaSeconds :type Float%20%28single-precision%29)))

(fn SpawnLoot
  (Game|SpawnActorfromClass (Utilities|ChooseLoot) (Math|Transform|MakeTransform (Transformation|GetActorLocation (Components|GetOwner)) "0, 0, 0" "1,1,1") "Undefined" 0 0))