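; InGame game-rules Blueprint that runs the match flow from player spawn through start, death respawn and end.
; BeginPlay marks Spawnpoint or StartPoint actors depending on the GameStart flag, spawns the player through Spawner and binds its death event.
; Player death respawns the player, calls a game reset and rebinds the event.
; Start and end events forward to their call functions, while GameTimer is an empty stub.
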(event Custom|Load%20Player
  ;[1 1 1] Pre Game
  (Default|SpawnPlayer (Variables|Default|GetSpawner)))

(event Custom|InitPlayer
  ;[1 1 1] Pre Game
  (bind _output_get (Variables|Default|SetPlayer (Game|GetPlayerCharacter 0)))
  (bind _asbase_player_character (Utilities|Casting|CastToBasePlayerCharacter _output_get))
  (EventDispatchers|BindEventtoPlayerDead _asbase_player_character (delegate Custom|DeathOfThePlayer)))

(event Custom|Game%20Timer
  ;[1 1 1] Pre Game
)

(event Custom|Game_Start
  ;[1 1 1] In Game
  (Default|CallStartGame))

(event Custom|GameEnd
  ;[1 1 1] Post Game
  (Default|CallEndGame))

(event Custom|RespawnPlayer
  ;[1 1 1] Gameplay Interactions
  (Default|SpawnPlayer (Variables|Default|GetSpawner))
  (Default|CallResetGame)
  (CallFunction|InitPlayer))

(event Custom|DeathOfThePlayer
  ;[1 1 1] Gameplay Interactions
  (CallFunction|RespawnPlayer))

(event EventBeginPlay
  ;[1 1 1] Pre Game
  (|BeginPlay))

(fn ConstructionScript)

(fn FindSpawnPoint
  (if (Variables|Default|GetGameStart)
    (bind _outactors (Actor|GetAllActorsOfClass "/Game/Blueprints/LevelObjects/GameRuleObjects/Spawnpoint.Spawnpoint_C"))
    (for _array_element _outactors
      (Default|SetSpawn _array_element))
    (else
      (bind _outactors_2 (Actor|GetAllActorsOfClass "/Game/Blueprints/LevelObjects/GameRuleObjects/StartPoint.StartPoint_C"))
      (for _array_element_2 _outactors_2
        (Default|SetSpawn _array_element_2)))))