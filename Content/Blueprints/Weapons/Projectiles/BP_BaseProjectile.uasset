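; Base projectile Blueprint for weapons that damages what it hits and explodes on impact.
; The sphere's hit event destroys the projectile silently, with no damage or effects, if it strikes the first player's character.
; Any other hit runs once through a DoOnce, applying Damage to that actor, spawning an explosion emitter and sound at the sphere's location, then destroying the projectile.
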(event OnComponentHit(Sphere)
  (params (HitComponent :type Primitive%20Component%20Object%20Reference) (OtherActor :type Actor%20Object%20Reference) (OtherComp :type Primitive%20Component%20Object%20Reference) (NormalImpulse :type Vector :default "0, 0, 0") (Hit :type Hit%20Result%20Structure%20%28by%20ref%29))
  (bind _sphere (Variables|Default|GetSphere))
  (bind _returnvalue (Transformation|GetWorldLocation _sphere))
  (if (== OtherActor (Game|GetPlayerCharacter 0))
    (Actor|DestroyActor)
    (else
      (Utilities|FlowControl|DoOnce false
        (:Completed
          (Game|Damage|ApplyDamage OtherActor (Variables|Default|GetDamage) 0 0)
          (Effects|SpawnEmitteratLocation "/Game/StarterContent/Particles/P_Explosion.P_Explosion" _returnvalue)
          (Audio|SpawnSoundatLocation "/Game/StarterContent/Audio/Explosion01.Explosion01" _returnvalue "0, 0, 0" 0.3 1.0 0.0 0 0)
          (Actor|DestroyActor))))))

(event EventBeginPlay)

(event Collision|EventActorBeginOverlap
  (params (OtherActor :type Actor%20Object%20Reference)))

(event EventTick
  (params (DeltaSeconds :type Float%20%28single-precision%29)))

(fn ConstructionScript)