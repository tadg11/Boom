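; Base handheld weapon that attaches its body mesh to the owning player's arms pose and fires projectiles from an aim arrow.
; A looping timer jitters the arrow toward random points around AimLoc to create spread.
; Trigger events branch on fire type via timers: semi-auto, full-auto, manual reload-per-shot, and a stubbed charge mode.
; Timed reloads draw from the player's rarity-indexed ammo pools, only when a full refill is available.
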(event Custom|OrientArrow
  (bind _weaponspread (Variables|Default|GetWeaponSpread))
  ;[1 1 1] Aiming
  (bind _output_get (Variables|Default|SetSpread%20Loc (Math|Random|RandomPointinBoundingBox (Variables|Default|GetAimLoc) (Math|Vector|MakeVector _weaponspread _weaponspread (+ _weaponspread 25.0)))))
  (Transformation|SetWorldRotation (Variables|Default|GetArrow) (Math|Rotator|FindLookatRotation (Transformation|GetWorldLocation (Variables|Default|GetArrow)) _output_get) false false))

(event Custom|EmptyFX
  (Audio|PlaySoundatLocation "/Game/SuperGrid/TutorialLevel/SoundEffects/MetalStepA.MetalStepA" (Transformation|GetActorLocation) "0, 0, 0" 0.7 1.0 0.0 0 0 0))

(event Custom|FireFX)

(event EventBeginPlay
  ;[1 1 1] Aiming
  (Utilities|Time|SetTimerbyEvent (delegate Custom|OrientArrow) 0.01 true)
  (Utilities|FlowControl|Delay 0.1)
  (bind _asbase_player_character (Utilities|Casting|CastToBasePlayerCharacter (Components|GetOwner)))
  (Variables|Default|SetPlayerOwner _asbase_player_character)
  (Class|SkinnedMeshComponent|SetMasterPoseComponent (Variables|Default|GetAnimBody) (Variables|/Game/Blueprints/Character/BasePlayerCharacter.BasePlayerCharacter_C|GetArms _asbase_player_character) false)
  (Variables|Default|SetAmmoCount (Utilities|Array|Get(acopy) (Variables|/Game/Blueprints/Character/BasePlayerCharacter.BasePlayerCharacter_C|GetMagazines _asbase_player_character) (Variables|/Game/Blueprints/Character/BasePlayerCharacter.BasePlayerCharacter_C|GetWeaponID _asbase_player_character))))

(event Collision|EventActorBeginOverlap
  (params (OtherActor :type Actor%20Object%20Reference)))

(event EventTick
  (params (DeltaSeconds :type Float%20%28single-precision%29)))

(fn ConstructionScript)

(fn Fire
  (bind _arrow (Variables|Default|GetArrow))
  (Math|Integer|DecrementInt (Variables|Default|GetAmmoCount)
    (:%20%20
      (bind _returnvalue (Game|SpawnActorfromClass (Variables|Default|GetProjectile) (Math|Transform|MakeTransform (+ (Transformation|GetWorldLocation _arrow) (* (Math|Vector|GetForwardVector _arrow) 75.0)) (Transformation|GetWorldRotation _arrow)) "Undefined" 0 0))
      (Collision|IgnoreActorwhenMoving (Variables|/Script/Engine.Character|GetCapsuleComponent (Variables|Default|GetPlayerOwner)) _returnvalue true)
      (Audio|PlaySoundatLocation "/Game/MovementAssets/Audio/fire_cue.fire_cue" (Transformation|GetActorLocation) "0, 0, 0" 0.3 1.0 0.0 0 0 0) ; Play firing sound
      (CallFunction|FireFX)
      (return))))

(fn ReloadCheck
  (bind _ammocount (Variables|Default|GetAmmoCount))
  (bind _maxammo (Variables|Default|GetMaxAmmo))
  (bind _playerowner (Variables|Default|GetPlayerOwner))
  (bind _returnvalue (- _maxammo _ammocount))
  (bind _ammo (Variables|/Game/Blueprints/Character/BasePlayerCharacter.BasePlayerCharacter_C|GetAmmo _playerowner))
  (bind _output (Utilities|Array|Get(acopy) _ammo 3))
  (bind _output_2 (Utilities|Array|Get(acopy) _ammo))
  (bind _output_3 (Utilities|Array|Get(acopy) _ammo 1))
  (bind _output_4 (Utilities|Array|Get(acopy) _ammo 2))
  (bind _returnvalue_2 (- _output_3 _returnvalue))
  (bind _returnvalue_3 (- _output_4 _returnvalue))
  (bind _returnvalue_4 (- _output _returnvalue))
  (bind _returnvalue_5 (- _output_2 _returnvalue))
  (switch Utilities|FlowControl|Switch|SwitchonWeaponRarity (Variables|Default|GetRarity)
    (:NewEnumerator0
      (if (> _returnvalue_5 -1)
        (Utilities|Array|SetArrayElem _ammo 0 _returnvalue_5)
        (return true)
        (else
          _)))
    (:NewEnumerator1
      (if (> _returnvalue_2 -1)
        (Utilities|Array|SetArrayElem _ammo 1 _returnvalue_2)
        (return true)
        (else
          _)))
    (:NewEnumerator2
      (if (> _returnvalue_3 -1)
        (Utilities|Array|SetArrayElem _ammo 2 _returnvalue_3)
        (return true)
        (else
          _)))
    (:NewEnumerator3
      (if (> _returnvalue_4 -1)
        (Utilities|Array|SetArrayElem _ammo 3 _returnvalue_4)
        (return true)
        (else
          _))))
  (return false))

(event Custom|ChamberRound
  (Variables|Default|SetCanShoot true)
  (Variables|Default|SetFiring false))

(event Custom|AutoFire
  (CallFunction|Fire))

(event Custom|BeginAuto
  (bind _returnvalue (Utilities|Time|SetTimerbyEvent (delegate Custom|AutoFire) (Variables|Default|GetFireRate) true))
  (Variables|Default|SetFullAutoTimer _returnvalue))

(event Custom|BeginCharge
  (Variables|Default|SetFiring false))

(event EventTriggerPull
  (if (Variables|Default|GetEmpty)
    (CallFunction|EmptyFX)
    (CallFunction|OutOfAmmo)
    (CallFunction|GunEmpty)
    (elif (Variables|Default|GetCanShoot)
      (Utilities|FlowControl|Sequence
        (:then_0
          (Variables|Default|SetCanShoot false))
        (:then_1
          (if (<= (Variables|Default|GetAmmoCount) 0)
            (CallFunction|OutOfAmmo)
            (else
              (Variables|Default|SetFiring true)
              (switch Utilities|FlowControl|Switch|SwitchonFireType (Variables|Default|GetFiretype)
                (:NewEnumerator0
                  (CallFunction|Fire)
                  (Utilities|Time|SetTimerbyEvent (delegate Custom|ChamberRound) (Variables|Default|GetFireRate)))
                (:NewEnumerator1
                  (CallFunction|BeginAuto))
                (:NewEnumerator2
                  (CallFunction|Fire)
                  (Variables|Default|SetFiring false)
                  (CallFunction|OutOfAmmo))
                (:NewEnumerator3
                  (CallFunction|BeginCharge)))))
          (if (<= (Variables|Default|GetAmmoCount) 0)
            (CallFunction|GunEmpty)))))))

(event Custom|Gun%20Empty
  (Variables|Default|SetEmpty true))

(event Custom|EndAuto
  (Utilities|Time|ClearandInvalidateTimerbyHandle (Variables|Default|GetFullAutoTimer))
  (Variables|Default|SetFullAutoTimer "")
  (Variables|Default|SetFiring false))

(event Custom|End%20Charge)

(event EventTriggerRelease
  (switch Utilities|FlowControl|Switch|SwitchonFireType (Variables|Default|GetFiretype)
    (:NewEnumerator1
      (CallFunction|EndAuto))
    (:NewEnumerator3
      (CallFunction|EndCharge))))

(event Custom|FillWithBullets
  (Variables|Default|SetAmmoCount (Variables|Default|GetMaxAmmo))
  (Utilities|Time|ClearandInvalidateTimerbyHandle (stale Custom|OutOfAmmo _returnvalue))
  (Variables|Default|SetCanShoot true)
  (Variables|Default|SetEmpty false)
  (Variables|Default|SetLoading false))

(event Custom|OutOfAmmo
  (Variables|Default|SetCanShoot false)
  (bind _success (CallFunction|ReloadCheck))
  (if _success
    (Variables|Default|SetLoading true)
    (bind _returnvalue (Utilities|Time|SetTimerbyEvent (delegate Custom|FillWithBullets) (Variables|Default|GetReloadTime)))
    (else
      (CallFunction|GunEmpty))))

(event EventLoadGun
  (Variables|Default|SetCanShoot false)
  (bind _success (CallFunction|ReloadCheck))
  (if _success
    (Variables|Default|SetLoading true)
    (bind _returnvalue (Utilities|Time|SetTimerbyEvent (delegate Custom|FillWithBullets) (Variables|Default|GetReloadTime)))
    (else
      (CallFunction|GunEmpty))))