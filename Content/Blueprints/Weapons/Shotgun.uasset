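; Shotgun weapon Blueprint whose Fire function spends one ammo to launch a burst of projectiles.
; Projectiles spawn at random points in a flat horizontal box ahead of the Arrow component, all sharing its rotation, so spread comes from position rather than angle.
; The owning player's capsule ignores each projectile when moving, then the firing sound and FireFX play once per shot.
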(event EventBeginPlay
  (|CallParentFunction) ; This node is disabled and will not be called.\nDrag off pins to build functionality.
)

(event Collision|EventActorBeginOverlap
  (params (OtherActor :type Actor%20Object%20Reference))
  (|CallParentFunction OtherActor) ; This node is disabled and will not be called.\nDrag off pins to build functionality.
)

(event EventTick
  (params (DeltaSeconds :type Float%20%28single-precision%29))
  (|CallParentFunction DeltaSeconds) ; This node is disabled and will not be called.\nDrag off pins to build functionality.
)

(fn ConstructionScript
  (|CallParentFunction))

(fn Fire
  (bind _arrow (Variables|Default|GetArrow))
  (Math|Integer|DecrementInt (Variables|Default|GetAmmoCount)
    (:%20%20
      (for _index (range 0 4)
        (bind _returnvalue (Game|SpawnActorfromClass (Variables|Default|GetProjectile) (Math|Transform|MakeTransform (Math|Random|RandomPointinBoundingBox (+ (Transformation|GetWorldLocation _arrow) (* (Math|Vector|GetForwardVector _arrow) 1e+02)) "100.000000,100.000000,0.000000") (Transformation|GetWorldRotation _arrow)) "Undefined" 0 0))
        (Collision|IgnoreActorwhenMoving (Variables|/Script/Engine.Character|GetCapsuleComponent (Variables|Default|GetPlayerOwner)) _returnvalue true))
      (Audio|PlaySoundatLocation "/Game/MovementAssets/Audio/fire_cue.fire_cue" (Transformation|GetActorLocation) "0, 0, 0" 0.5 1.0 0.0 0 0 0) ; Play firing sound
      (CallFunction|FireFX)
      (return))))