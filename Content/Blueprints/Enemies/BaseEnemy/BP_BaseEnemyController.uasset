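; Base enemy AI controller that runs the BT_BaseEnemy behavior tree and links perception to its blackboard.
; Perception updates set PlayerSpotted when a BasePlayerCharacter is sensed or lost.
; A fast looping timer focuses the player while InCombat is true.
; Losing sight, or each update outside combat, sets a randomized cooldown timer that clears InCombat and also focuses the player.
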(event OnTargetPerceptionUpdated(AIPerception)
  (params (Actor :type Actor%20Object%20Reference) (Stimulus :type AI%20Stimulus%20Structure))
  (bind _returnvalue (AI|GetBlackboard 0))
  (bind _returnvalue_2 (Utilities|Name|MakeLiteralName "PlayerSpotted"))
  ;[1 1 1] Perception
  (if (== (Utilities|GetClass Actor) "/Game/Blueprints/Character/BasePlayerCharacter.BasePlayerCharacter_C")
    (if (.bSuccessfullySensed (Utilities|Struct|BreakAIStimulus Stimulus))
      (AI|Components|Blackboard|SetValueasBool _returnvalue _returnvalue_2 true)
      (else
        (AI|Components|Blackboard|SetValueasBool _returnvalue _returnvalue_2 false)
        ;[1 1 1] Begin Play & Updates
        (bind _returnvalue_3 (Utilities|Time|SetTimerbyEvent (delegate Custom|Combat%20Cooldown) (Math|Random|RandomFloatinRange 5.0 7.0)))))))

(event Custom|Update
  ;[1 1 1] Begin Play & Updates
  (bind _output_get (Variables|Default|SetInCombat (ScalableFloat|GetValueasBool (AI|GetBlackboard self) (Utilities|Name|MakeLiteralName "InCombat"))))
  (if _output_get
    (AI|SetFocus (Game|GetPlayerCharacter 0))
    (else
      (bind _returnvalue (Utilities|Time|SetTimerbyEvent (delegate Custom|Combat%20Cooldown) (Math|Random|RandomFloatinRange 5.0 7.0))))))

(event Custom|Combat%20Cooldown
  ;[1 1 1] Begin Play & Updates
  (AI|Components|Blackboard|SetValueasBool (Variables|/Script/AIModule.AIController|GetBlackboard self) (Utilities|Name|MakeLiteralName "InCombat") false)
  (Utilities|Time|ClearandInvalidateTimerbyHandle (stale OnTargetPerceptionUpdated(AIPerception) _returnvalue_3))
  (AI|SetFocus (Game|GetPlayerCharacter 0)))

(event EventBeginPlay
  ;[1 1 1] Begin Play & Updates
  (AI|RunBehaviorTree "/Game/Blueprints/Enemies/BaseEnemy/BT_BaseEnemy.BT_BaseEnemy")
  (Utilities|Time|SetTimerbyEvent (delegate Custom|Update) 0.01 true))

(event EventTick
  (params (DeltaSeconds :type Float%20%28single-precision%29)))

(fn ConstructionScript)