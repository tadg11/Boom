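; Base enemy character with timed melee attacks, pain reactions, death and loot drops.
; A looping timer mirrors the blackboard's InCombat flag, while attack, pain and death events set state flags and walk speed.
; Attacks damage the player after a delay if still within range.
; Death clears combat state, waits, spawns LootTable1 loot, calls DeadEnemy and destroys the actor.
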(event OnComponentHit(CapsuleComponent)
  (params (HitComponent :type Primitive%20Component%20Object%20Reference) (OtherActor :type Actor%20Object%20Reference) (OtherComp :type Primitive%20Component%20Object%20Reference) (NormalImpulse :type Vector :default "0, 0, 0") (Hit :type Hit%20Result%20Structure%20%28by%20ref%29)))

(event Custom|Update
  ;[1 1 1] Update & Begin Play
  (Variables|Default|SetInCombat (ScalableFloat|GetValueasBool (AI|GetBlackboard (Pawn|GetController)) (Utilities|Name|MakeLiteralName "InCombat"))))

(event Custom|AttackStart
  (bind _returnvalue (Game|GetPlayerCharacter 0))
  (Variables|/Script/Engine.CharacterMovementComponent|SetMaxWalkSpeed (Variables|Character|GetCharacterMovement) 1.5e+02)
  (Variables|Default|SetAttacking true)
  (bind _returnvalue_2 (Utilities|Time|SetTimerbyEvent (delegate Custom|AttackEnd) 1.145))
  (Utilities|FlowControl|Delay 1.0)
  (if (<= (Math|Vector|Distance(Vector) (Transformation|GetActorLocation _returnvalue) (Transformation|GetActorLocation)) 2e+02)
    (bind _returnvalue_3 (Game|Damage|ApplyDamage _returnvalue 1e+01 0 self))
    (Development|PrintString (Utilities|String|ToString(Float) _returnvalue_3))))

(event Custom|AttackEnd
  (Variables|/Script/Engine.CharacterMovementComponent|SetMaxWalkSpeed (Variables|Character|GetCharacterMovement) 5e+02)
  (Variables|Default|SetAttacking false)
  (Utilities|Time|ClearandInvalidateTimerbyHandle (stale Custom|AttackStart _returnvalue_2)))

(event EventBeginPlay
  ;[1 1 1] Update & Begin Play
  (Utilities|Time|SetTimerbyEvent (delegate Custom|Update) 0.01 true))

(event Collision|EventActorBeginOverlap
  (params (OtherActor :type Actor%20Object%20Reference)))

(event EventTick
  (params (DeltaSeconds :type Float%20%28single-precision%29)))

(fn ConstructionScript)

(event Custom|EnemyDeath
  (AI|Components|Blackboard|SetValueasBool (AI|GetBlackboard (AI|GetAIController self)) (Utilities|Name|MakeLiteralName "InCombat") false)
  (Variables|Default|SetInCombat false)
  (Variables|Default|SetDead true)
  (Utilities|FlowControl|Delay 2.14)
  (Default|SpawnLoot (Variables|Default|GetLootTable1))
  (Default|CallDeadEnemy)
  (Actor|DestroyActor))

(event Game|Damage|EventAnyDamage
  (params (Damage :type Float%20%28single-precision%29) (DamageType :type Damage%20Type%20Object%20Reference) (InstigatedBy :type Controller%20Object%20Reference) (DamageCauser :type Actor%20Object%20Reference))
  (bind _charactermovement (Variables|Character|GetCharacterMovement))
  (Variables|Default|SetPain true)
  (Variables|/Script/Engine.CharacterMovementComponent|SetMaxWalkSpeed _charactermovement 1.0)
  (Utilities|FlowControl|Delay 0.29)
  (Variables|/Script/Engine.CharacterMovementComponent|SetMaxWalkSpeed _charactermovement 5e+02)
  (Variables|Default|SetPain false)
  (bind _output_get (Variables|Default|SetHealth (- (Variables|Default|GetHealth) Damage)))
  (if (<= _output_get 0.0)
    (Variables|/Script/Engine.CharacterMovementComponent|SetMaxWalkSpeed _charactermovement 25.0)
    (CallFunction|EnemyDeath)))